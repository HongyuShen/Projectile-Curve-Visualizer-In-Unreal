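; Actor that previews a projectile's arc as a spline mesh with a target marker aligned to the predicted hit surface.
; VisualizeProjectileCurve runs a predicted path trace and fits a two-point spline with computed tangents, drawing a straight line for two samples and hiding itself without a valid hit.
; A target-location variant leads the target using target and thrower velocities, solves the toss velocity, then feeds that visualizer.
; Helpers handle hiding and mesh scaling.
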(fn ConstructionScript
  (bind _returnvalue (AddComponent|AddSplineMeshComponent false))
  (Variables|Default|SetProjectileCurveSplineMesh _returnvalue))

(fn SetProjectileCurveSplineMeshScale
  (params (Scale :type Vector))
  (Transformation|SetRelativeScale3D (Variables|Default|GetProjectileCurveSplineMesh) Scale))

(fn SetProjectileTargetStaticMeshScale
  (params (Scale :type Vector))
  (Transformation|SetRelativeScale3D (Variables|Default|GetProjectileTargetStaticMesh) Scale))

(fn VisualizeProjectileCurve
  (params (ProjectileStartLocation :type Vector) (ProjectileStartLocationForwardOffset :type Float%20%28single-precision%29) (LaunchVelocity :type Vector) (ProjectileRadius :type Float%20%28single-precision%29) (TraceChannel :type ECollisionChannel%20Enum :default "ECC_WorldStatic") (DistanceOffsetAboveHitLocation :type Float%20%28single-precision%29) (PredictProjectileDrawDebugType :type EDrawDebugTrace%20Enum :default "None"))
  (bind _returnvalue (Math|Vector|Normalize LaunchVelocity))
  (bind _returnvalue_2 (Transformation|GetActorLocation))
  (bind _projectilecurvespline (Variables|Default|GetProjectileCurveSpline))
  (bind _projectilecurvesplinemesh (Variables|Default|GetProjectileCurveSplineMesh))
  (bind _projectilecurvespline_2 (Variables|Default|GetProjectileCurveSpline))
  (bind _projectilecurvesplinemesh_2 (Variables|Default|GetProjectileCurveSplineMesh))
  (bind _projectiletargetstaticmesh (Variables|Default|GetProjectileTargetStaticMesh))
  (bind _returnvalue_3 (* (Math|Vector|MakeVector (.x _returnvalue) (.y _returnvalue) 0.0) ProjectileStartLocationForwardOffset))
  (bind _returnvalue_4 (Transformation|GetWorldLocation _projectiletargetstaticmesh))
  (bind (_location _tangent) (Spline|GetLocationandTangentatSplinePoint _projectilecurvespline 1 "Local"))
  (bind (_location_2 _tangent_2) (Spline|GetLocationandTangentatSplinePoint _projectilecurvespline 0 "Local"))
  (bind _returnvalue_5 (+ _returnvalue_2 LaunchVelocity))
  (bind _returnvalue_6 (Math|Rotator|FindLookatRotation _returnvalue_2 _returnvalue_5))
  (bind _returnvalue_7 (+ ProjectileStartLocation _returnvalue_3))
  (if (not (Rendering|IsVisible _projectilecurvesplinemesh_2))
    (Rendering|SetVisibility _projectilecurvesplinemesh_2 true false))
  (bind (_outhit _outpathpositions _outlasttracedestination _returnvalue_8) (Class|GameplayStatics|BlueprintPredictProjectilePathbyTraceChannel _returnvalue_7 LaunchVelocity true ProjectileRadius TraceChannel false 0 PredictProjectileDrawDebugType 0.0 3.0))
  (if _returnvalue_8
    (if (> (Utilities|Array|Length _outpathpositions) 2)
      ;[1 1 1] At least 3 points to form a curve
      (Transformation|SetActorLocationAndRotation _returnvalue_7 (Math|Rotator|MakeRotator 0.0 0.0 (.yaw _returnvalue_6)))
      (Spline|SetLocationatSplinePoint _projectilecurvespline_2 0 (Utilities|Array|Get(acopy) _outpathpositions) "World" false)
      (Spline|SetTangentatSplinePoint _projectilecurvespline_2 0 (Math|Vector|MakeVector (* (Math|Vector|Distance2D(Vector) (Math|Vector2D|MakeVector2D (.x (- (- (* (Utilities|Array|Get(acopy) _outpathpositions 1) 2.0) (* (Utilities|Array|Get(acopy) _outpathpositions) 0.5)) (* (Utilities|Array|Get(acopy) _outpathpositions (- (Utilities|Array|Length _outpathpositions) 1)) 0.5))) (.y (- (- (* (Utilities|Array|Get(acopy) _outpathpositions 1) 2.0) (* (Utilities|Array|Get(acopy) _outpathpositions) 0.5)) (* (Utilities|Array|Get(acopy) _outpathpositions (- (Utilities|Array|Length _outpathpositions) 1)) 0.5)))) (Math|Vector2D|MakeVector2D (.X (Math|Vector|BreakVector (Utilities|Array|Get(acopy) _outpathpositions))) (.Y (Math|Vector|BreakVector (Utilities|Array|Get(acopy) _outpathpositions))))) 2.0) 0.0 (* (- (.Z (Math|Vector|BreakVector (Utilities|Array|Get(acopy) _outpathpositions))) (.z (- (- (* (Utilities|Array|Get(acopy) _outpathpositions 1) 2.0) (* (Utilities|Array|Get(acopy) _outpathpositions) 0.5)) (* (Utilities|Array|Get(acopy) _outpathpositions (- (Utilities|Array|Length _outpathpositions) 1)) 0.5)))) -2.0)) "Local" false)
      (Spline|SetLocationatSplinePoint _projectilecurvespline_2 1 (Utilities|Array|Get(acopy) _outpathpositions (- (Utilities|Array|Length _outpathpositions) 1)) "World" false)
      (Spline|SetTangentatSplinePoint _projectilecurvespline_2 1 (Math|Vector|MakeVector (* (Math|Vector|Distance2D(Vector) (Math|Vector2D|MakeVector2D (.x (- (- (* (Utilities|Array|Get(acopy) _outpathpositions 1) 2.0) (* (Utilities|Array|Get(acopy) _outpathpositions) 0.5)) (* (Utilities|Array|Get(acopy) _outpathpositions (- (Utilities|Array|Length _outpathpositions) 1)) 0.5))) (.y (- (- (* (Utilities|Array|Get(acopy) _outpathpositions 1) 2.0) (* (Utilities|Array|Get(acopy) _outpathpositions) 0.5)) (* (Utilities|Array|Get(acopy) _outpathpositions (- (Utilities|Array|Length _outpathpositions) 1)) 0.5)))) (Math|Vector2D|MakeVector2D (.X (Math|Vector|BreakVector (Utilities|Array|Get(acopy) _outpathpositions (- (Utilities|Array|Length _outpathpositions) 1)))) (.Y (Math|Vector|BreakVector (Utilities|Array|Get(acopy) _outpathpositions (- (Utilities|Array|Length _outpathpositions) 1)))))) 2.0) 0.0 (* (- (.Z (Math|Vector|BreakVector (Utilities|Array|Get(acopy) _outpathpositions (- (Utilities|Array|Length _outpathpositions) 1)))) (.z (- (- (* (Utilities|Array|Get(acopy) _outpathpositions 1) 2.0) (* (Utilities|Array|Get(acopy) _outpathpositions) 0.5)) (* (Utilities|Array|Get(acopy) _outpathpositions (- (Utilities|Array|Length _outpathpositions) 1)) 0.5)))) 2.0)) "Local" true)
      (SplineMesh|SetStartandEnd (Variables|Default|GetProjectileCurveSplineMesh) _location_2 _tangent_2 _location _tangent true :!class /Script/Engine.SplineMeshComponent :!label _label)
      (Transformation|SetWorldLocationAndRotation _projectiletargetstaticmesh (+ (.Location (Collision|BreakHitResult _outhit)) (* (.Normal (Collision|BreakHitResult _outhit)) DistanceOffsetAboveHitLocation)) (Math|Rotator|FindLookatRotation _returnvalue_4 (+ _returnvalue_4 (.Normal (Collision|BreakHitResult _outhit)))) false false)
      (if (not (Rendering|IsVisible _projectiletargetstaticmesh))
        (Rendering|SetVisibility _projectiletargetstaticmesh true false))
      (return _returnvalue_7 "" _returnvalue_8)
      (elif (== (Utilities|Array|Length _outpathpositions) 2)
        ;[1 1 1] Form a straight line if only has 2 points
        (Transformation|SetActorLocationAndRotation _returnvalue_7 (Math|Rotator|MakeRotator 0.0 0.0 (.yaw _returnvalue_6)))
        (Spline|SetLocationatSplinePoint _projectilecurvespline_2 0 (Utilities|Array|Get(acopy) _outpathpositions) "World" false)
        (Spline|SetTangentatSplinePoint _projectilecurvespline_2 0 (Math|Vector|MakeVector 0.0 0.0 0.0) "Local" false)
        (Spline|SetLocationatSplinePoint _projectilecurvespline_2 1 (Utilities|Array|Get(acopy) _outpathpositions (- (Utilities|Array|Length _outpathpositions) 1)) "World" false)
        (Spline|SetTangentatSplinePoint _projectilecurvespline_2 1 (Math|Vector|MakeVector 0.0 0.0 0.0) "Local" true)
        (goto _label)
        (else
          _))))
  ;[1 1 1] Otherwise no curve/straight line is shown
  (if (Rendering|IsVisible _projectilecurvesplinemesh)
    (Rendering|SetVisibility _projectilecurvesplinemesh false false)
    (Rendering|SetVisibility (Variables|Default|GetProjectileTargetStaticMesh) false false))
  (return "0, 0, 0" "" false))

(fn VisualizeProjectileCurvewithTargetLocation
  (params (ProjectileStartLocation :type Vector) (ProjectileStartLocationForwardOffset :type Float%20%28single-precision%29) (ProjectileEndLocation :type Vector) (ProjectileLaunchSpeed :type Float%20%28single-precision%29) (ThrowerVelocity :type Vector) (TargetActorVelocity :type Vector) (ProjectileRadius :type Float%20%28single-precision%29) (TraceChannel :type ECollisionChannel%20Enum :default "ECC_WorldStatic") (DistanceOffsetAboveHitLocation :type Float%20%28single-precision%29) (PredictProjectileDrawDebugType :type EDrawDebugTrace%20Enum :default "None"))
  (bind _returnvalue (Math|Vector|Distance(Vector) ProjectileStartLocation ProjectileEndLocation))
  (bind _returnvalue_2 (/ _returnvalue ProjectileLaunchSpeed))
  (bind _returnvalue_3 (* TargetActorVelocity _returnvalue_2))
  (bind _returnvalue_4 (* _returnvalue_2 -1.0))
  (bind _returnvalue_5 (* ThrowerVelocity _returnvalue_4))
  (bind _returnvalue_6 (+ _returnvalue_3 _returnvalue_5))
  (bind _returnvalue_7 (+ ProjectileEndLocation _returnvalue_6))
  (bind _returnvalue_8 (- _returnvalue_7 ProjectileStartLocation))
  (bind _returnvalue_9 (Math|Vector|Normalize _returnvalue_8))
  (bind _returnvalue_10 (* (Math|Vector|MakeVector (.x _returnvalue_9) (.y _returnvalue_9) 0.0) ProjectileStartLocationForwardOffset))
  (bind _returnvalue_11 (+ ProjectileStartLocation _returnvalue_10))
  (bind (_tossvelocity _returnvalue_12) (Class|GameplayStatics|BlueprintSuggestProjectileVelocity _returnvalue_11 _returnvalue_7 ProjectileLaunchSpeed 0.0 "DoNotTrace" 0.0 false false))
  (if _returnvalue_12
    (bind (_updatedprojectilestartlocation _hitresult _hit) (CallFunction|VisualizeProjectileCurve _returnvalue_11 0.0 _tossvelocity ProjectileRadius TraceChannel DistanceOffsetAboveHitLocation PredictProjectileDrawDebugType))
    (return _updatedprojectilestartlocation _tossvelocity _returnvalue_7 _hitresult _hit)
    (else
      (return "0, 0, 0" "0, 0, 0" "0, 0, 0" "" false))))

(fn HideProjectileCurve
  (params (HideTargetOnly :type Boolean))
  (bind _projectilecurvesplinemesh (Variables|Default|GetProjectileCurveSplineMesh))
  (bind _projectiletargetstaticmesh (Variables|Default|GetProjectileTargetStaticMesh))
  (if HideTargetOnly
    (if (Rendering|IsVisible _projectiletargetstaticmesh)
      (Rendering|SetVisibility _projectiletargetstaticmesh false false :!label _label)
      (Collision|SetCollisionEnabled _projectiletargetstaticmesh "NoCollision"))
    (elif (Rendering|IsVisible _projectilecurvesplinemesh)
      (Rendering|SetVisibility _projectilecurvesplinemesh false false)
      (goto _label))))